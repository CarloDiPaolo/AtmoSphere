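; Level trigger actor that restarts the current level when the player pawn overlaps it, named for use as a fall catch.
; On overlap, it fades the camera out over FadeDuration, waits for that delay, then reopens the current level by name.
; BeginPlay fades the camera in from full, and the overlap chain also wires into that same fade after the level open call.
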(event OnComponentBeginOverlap(Trigger)
  (params (OverlappedComponent :type Primitive%20Component%20Object%20Reference) (OtherActor :type Actor%20Object%20Reference) (OtherComp :type Primitive%20Component%20Object%20Reference) (OtherBodyIndex :type Integer) (bFromSweep :type Boolean) (SweepResult :type Hit%20Result%20Structure%20%28by%20ref%29))
  (bind _returnvalue (Game|GetPlayerCameraManager 0))
  (bind _fade_duration (Variables|Default|GetFade_Duration))
  (if (== OtherActor (Game|Player|GetPlayerPawn 0))
    (CameraFades|StartCameraFade :self _returnvalue :ToAlpha 1.0 :Duration _fade_duration :bHoldWhenFinished true)
    (Utilities|FlowControl|Delay _fade_duration)
    (bind _returnvalue_2 (Game|GetCurrentLevelName true))
    (Game|OpenLevel(byName) (Utilities|String|StringToName _returnvalue_2))
    (CameraFades|StartCameraFade :self _returnvalue :FromAlpha 1.0 :ToAlpha 0.0 :Duration 3.0)))

(event EventBeginPlay
  (CameraFades|StartCameraFade :self (Game|GetPlayerCameraManager 0) :FromAlpha 1.0 :ToAlpha 0.0 :Duration 3.0))

(event Collision|EventActorBeginOverlap
  (params (OtherActor :type Actor%20Object%20Reference)))

(event EventTick
  (params (DeltaSeconds :type Float%20%28single-precision%29)))

(fn ConstructionScript)