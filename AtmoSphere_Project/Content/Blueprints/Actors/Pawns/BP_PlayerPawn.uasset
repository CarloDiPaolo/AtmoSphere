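; BP_PlayerPawn is a player pawn that rolls a physics sphere relative to the camera.
; Both movement axes feed one AddTorqueInRadians call on MeshSphere, built from the camera's right and forward vectors flattened to horizontal and scaled by TorqueMultiplier.
; Mouse X yaws the spring arm to turn the view.
; An actor-rotation snippet following control yaw is left unconnected.
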(event EventBeginPlay)

(event Collision|EventActorBeginOverlap
  (params (OtherActor :type Actor%20Object%20Reference)))

(event EventTick
  (params (DeltaSeconds :type Float%20%28single-precision%29)))

(event Input|AxisEvents|InputAxisMoveForwards/Backwards
  (params (AxisValue :type Float%20%28single-precision%29))
  (bind _torque_multiplier (Variables|Default|GetTorque%20Multiplier))
  (bind _camera (Variables|Default|GetCamera))
  (bind _returnvalue (Math|Vector|GetForwardVector _camera))
  (bind _returnvalue_2 (Math|Vector|GetRightVector _camera))
  (bind (_x _y) (Math|Vector|BreakVector _returnvalue_2))
  (bind (_x_2 _y_2) (Math|Vector|BreakVector _returnvalue))
  ;[1 1 1] Camera Based Movement
  (Class|PrimitiveComponent|AddTorqueinRadians (Variables|Default|Getmesh_Sphere) (+ (* (Math|Vector|MakeVector _x _y 0.0) (* AxisValue _torque_multiplier)) (* (Math|Vector|MakeVector _x_2 _y_2 0.0) (* (stale Input|AxisEvents|InputAxisMoveLeft/Right AxisValue) _torque_multiplier))) "None" false))

(event Input|AxisEvents|InputAxisMoveLeft/Right
  (params (AxisValue :type Float%20%28single-precision%29))
  (bind _torque_multiplier (Variables|Default|GetTorque%20Multiplier))
  (bind _camera (Variables|Default|GetCamera))
  (bind _returnvalue (Math|Vector|GetForwardVector _camera))
  (bind _returnvalue_2 (Math|Vector|GetRightVector _camera))
  (bind (_x _y) (Math|Vector|BreakVector _returnvalue_2))
  (bind (_x_2 _y_2) (Math|Vector|BreakVector _returnvalue))
  ;[1 1 1] Camera Based Movement
  (Class|PrimitiveComponent|AddTorqueinRadians (Variables|Default|Getmesh_Sphere) (+ (* (Math|Vector|MakeVector _x _y 0.0) (* (stale Input|AxisEvents|InputAxisMoveForwards/Backwards AxisValue) _torque_multiplier)) (* (Math|Vector|MakeVector _x_2 _y_2 0.0) (* AxisValue _torque_multiplier))) "None" false))

(event Input|MouseEvents|MouseX
  (params (AxisValue :type Float%20%28single-precision%29))
  ;[1 1 1] Mouse Look
  (Transformation|AddLocalRotation (Variables|Default|GetSpringArm) (Math|Rotator|MakeRotator 0.0 0.0 AxisValue) false false))

(fn ConstructionScript)