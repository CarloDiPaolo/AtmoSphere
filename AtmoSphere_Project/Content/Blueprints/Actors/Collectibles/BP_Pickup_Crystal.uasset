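; Collectible crystal pickup actor that flies into the player and vanishes when the player overlaps it.
; On overlap it caches its location, scale and point light intensity, then plays CollectionTimeline.
; The timeline's curves drive lerps that pull it toward the pawn's live position, shrink it to zero and fade its light.
; The actor destroys itself when the timeline finishes, with no score or inventory update in this Blueprint.
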(event Collision|EventActorBeginOverlap
  (params (OtherActor :type Actor%20Object%20Reference))
  (Utilities|IsPlayer OtherActor
    (:IsPlayer
      (CallFunction|StoreStartingValues)
      (bind (_direction _location_anim _scale_anim _light_intensity_anim) (Timeline|Collection%20Timeline Play)
        (:Update
          (CallFunction|MovetoPlayer _location_anim)
          (CallFunction|ScaleCrystal _scale_anim)
          (CallFunction|AdjustLightIntensity _light_intensity_anim))
        (:Finished
          (Actor|DestroyActor))))))

(fn ConstructionScript)

(fn MovetoPlayer
  (params (Alpha :type Float%20%28single-precision%29))
  (Transformation|SetActorLocation (Math|Vector|Lerp(Vector) (Variables|Default|GetStart_Location) (Transformation|GetActorLocation (Game|Player|GetPlayerPawn 0)) Alpha) false false))

(fn StoreStartingValues
  (Variables|Default|SetStart_Location (Transformation|GetActorLocation))
  (Variables|Default|SetStart_Scale (Transformation|GetActorScale3D))
  (Variables|Default|SetPoint_Light_Intensity (Variables|/Script/Engine.LightComponentBase|GetIntensity (Variables|Default|GetPointLight))))

(fn ScaleCrystal
  (params (Alpha :type Float%20%28single-precision%29))
  (Transformation|SetActorScale3D (Math|Vector|Lerp(Vector) (Variables|Default|GetStart_Scale) "0, 0, 0" Alpha)))

(fn AdjustLightIntensity
  (params (Alpha :type Float%20%28single-precision%29))
  (Rendering|Components|Light|SetIntensity (Variables|Default|GetPointLight) (Math|Float|Lerp (Variables|Default|GetPoint_Light_Intensity) 0.0 Alpha)))