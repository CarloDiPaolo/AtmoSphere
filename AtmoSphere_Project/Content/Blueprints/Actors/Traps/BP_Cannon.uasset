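; Trap cannon that fires projectiles automatically on a repeating interval after an initial start delay.
; A spawn timeline creates a BP_Projectile_Static at the muzzle point on every update, scaled from zero toward full size to show the shot growing.
; When it finishes, the cannon spawns the real BP_Projectile and a second timeline moves the barrel along local Y.
; That timeline's Cannon Fired event restarts the interval delay, closing the loop.
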(event EventBeginPlay
  (bind _projectile_spawn (Variables|Default|GetProjectile_Spawn))
  (bind _returnvalue (Transformation|GetWorldLocation _projectile_spawn))
  (bind _returnvalue_2 (Transformation|GetWorldRotation _projectile_spawn))
  (Utilities|FlowControl|Delay (Variables|CannonTimings|GetStart_Delay))
  (Utilities|FlowControl|Delay (Variables|CannonTimings|GetInterval) :!label _label)
  (bind _float_scale_timeline (Timeline|Projectile_Spawn_Timline PlayFromStart)
    (:Update
      (Game|SpawnActorfromClass "/Game/Blueprints/Actors/Projectiles/BP_Projectile_Static.BP_Projectile_Static_C" (Math|Transform|MakeTransform _returnvalue _returnvalue_2 (Math|Conversions|ToVector(Float) (Math|Float|Lerp 0.0 1.0 _float_scale_timeline))) "AlwaysSpawn" 0 0))
    (:Finished
      (Game|SpawnActorfromClass "/Game/Blueprints/Actors/Projectiles/BP_Projectile.BP_Projectile_C" (Math|Transform|MakeTransform _returnvalue _returnvalue_2 (Transformation|GetWorldScale _projectile_spawn)) "AlwaysSpawn" 0 0)
      (bind _barrel_location (Timeline|CannonFire_Timeline PlayFromStart)
        (:Update
          (Transformation|SetRelativeLocation (Variables|Default|GetBarrel) (Math|Vector|MakeVector 0.0 _barrel_location 0.0) false false))
        (:Cannon_Fired
          (goto _label))))))

(event Collision|EventActorBeginOverlap
  (params (OtherActor :type Actor%20Object%20Reference)))

(event EventTick
  (params (DeltaSeconds :type Float%20%28single-precision%29)))

(fn ConstructionScript)